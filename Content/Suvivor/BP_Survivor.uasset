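; Survivor actor that takes damage through a health component and pauses the game when it dies.
; On BeginPlay it registers as a Game Framework Component Manager receiver, allowing modular component injection, and binds to its own any-damage event.
; Unless GodMode is set, incoming damage is truncated to an integer and passed to the HealthComponent, whose OnDeath event triggers the pause.
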(event `self.ReceiveBeginPlay`
  (`GameFrameworkComponentManager.AddReceiver` (subsystem `GameFrameworkComponentManager`) null true)
  (add `self.OnTakeAnyDamage` (delegate `OnTakeAnyDamage_Event`)))

(event `OnTakeAnyDamage_Event` :!signature `self.OnTakeAnyDamage`
  (params (DamagedActor :type "Actor Object Reference") (Damage :type "Float (single-precision)") (DamageType :type "DamageType Object Reference") (InstigatedBy :type "Controller Object Reference") (DamageCauser :type "Actor Object Reference"))
  (if (not (`self.GodMode`))
    (`HealthComponent.TakeDamage` (`self.HealthComponent`) (`KismetMathLibrary.FTrunc` Damage))))

(event `self.HealthComponent.OnDeath`
  (`GameplayStatics.SetGamePaused` true))

(fn `UserConstructionScript`)